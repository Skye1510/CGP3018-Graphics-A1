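; BP_Pedestal is a placement point where the third-person character can set down an orb.
; Overlapping its Box sets the character's CanPlace flag and NearbyPedestal reference, and leaving clears both.
; TryPlaceOrb accepts a held orb only while no valid orb is placed, stores it as PlacedOrb and calls PlaceOnPedestal on it.
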(event `self.Box.OnComponentBeginOverlap`
  (params (OverlappedComponent :type "PrimitiveComponent Object Reference") (OtherActor :type "Actor Object Reference") (OtherComp :type "PrimitiveComponent Object Reference") (OtherBodyIndex :type Integer) (bFromSweep :type Boolean) (SweepResult :type "HitResult Structure (by ref)"))
  (bind _asbp_third_person_character (cast `/Game/ThirdPerson/Blueprints/BP_ThirdPersonCharacter` OtherActor))
  (set `/Game/ThirdPerson/Blueprints/BP_ThirdPersonCharacter.bCanPlace` true _asbp_third_person_character)
  (set `/Game/ThirdPerson/Blueprints/BP_ThirdPersonCharacter.nearbyPedestal` self _asbp_third_person_character))

(event `self.Box.OnComponentEndOverlap`
  (params (OverlappedComponent :type "PrimitiveComponent Object Reference") (OtherActor :type "Actor Object Reference") (OtherComp :type "PrimitiveComponent Object Reference") (OtherBodyIndex :type Integer))
  (bind _asbp_third_person_character (cast `/Game/ThirdPerson/Blueprints/BP_ThirdPersonCharacter` OtherActor))
  (set `/Game/ThirdPerson/Blueprints/BP_ThirdPersonCharacter.bCanPlace` false _asbp_third_person_character)
  (set `/Game/ThirdPerson/Blueprints/BP_ThirdPersonCharacter.nearbyPedestal` null _asbp_third_person_character))

(event `TryPlaceOrb`
  (params (OrbToPlace :type "/Game/MyBlueprints/BP_ObjectPickup Object Reference"))
  (if (`KismetSystemLibrary.IsValid` (`self.PlacedOrb`))
    _
    (elif (`/Game/MyBlueprints/BP_ObjectPickup.bIsHeld` OrbToPlace)
      (set `self.PlacedOrb` OrbToPlace)
      (`/Game/MyBlueprints/BP_ObjectPickup.PlaceOnPedestal` OrbToPlace self))))

(fn `UserConstructionScript`)