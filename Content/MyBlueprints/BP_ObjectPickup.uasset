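; Color puzzle orb that the third-person character carries in its hand, drops or places on pedestals to open colored walls.
; Overlap registers it as the character's nearby orb; placing or removing it updates the character's PlacedOrbs list.
; Color then sums red, green and blue tags as bit values, hiding and disabling collision on PuzzleWall actors tagged with the mixed color.
; An older, disconnected copy of that logic remains in the EventGraph.
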(event `Drop`
  (`self.K2_DetachFromActor` "KeepWorld" "KeepWorld" "KeepWorld")
  (set `self.bIsHeld` false)
  (`PrimitiveComponent.SetCollisionEnabled` (`self.Sphere`) "QueryAndPhysics"))

(event `self.PickupCollider.OnComponentEndOverlap`
  (params (OverlappedComponent :type "PrimitiveComponent Object Reference") (OtherActor :type "Actor Object Reference") (OtherComp :type "PrimitiveComponent Object Reference") (OtherBodyIndex :type Integer))
  (bind _asbp_third_person_character (cast `/Game/ThirdPerson/Blueprints/BP_ThirdPersonCharacter` OtherActor))
  (set `/Game/ThirdPerson/Blueprints/BP_ThirdPersonCharacter.bCanPickup` false _asbp_third_person_character)
  (set `/Game/ThirdPerson/Blueprints/BP_ThirdPersonCharacter.nearbyOrb` null _asbp_third_person_character))

(event `self.PickupCollider.OnComponentBeginOverlap`
  (params (OverlappedComponent :type "PrimitiveComponent Object Reference") (OtherActor :type "Actor Object Reference") (OtherComp :type "PrimitiveComponent Object Reference") (OtherBodyIndex :type Integer) (bFromSweep :type Boolean) (SweepResult :type "HitResult Structure (by ref)"))
  (bind _asbp_third_person_character (cast `/Game/ThirdPerson/Blueprints/BP_ThirdPersonCharacter` OtherActor))
  (set `/Game/ThirdPerson/Blueprints/BP_ThirdPersonCharacter.bCanPickup` true _asbp_third_person_character)
  (set `/Game/ThirdPerson/Blueprints/BP_ThirdPersonCharacter.nearbyOrb` self _asbp_third_person_character))

(event `Pickup`
  (bind _currentpedestal (`self.CurrentPedestal`))
  (set `self.bIsHeld` true)
  (if (`KismetSystemLibrary.IsValid` _currentpedestal)
    (`self.K2_DetachFromActor` _currentpedestal "KeepRelative" "KeepRelative" "KeepRelative")
    (set `/Game/MyBlueprints/BP_Pedestal.PlacedOrb` null _currentpedestal)
    (set `self.CurrentPedestal` null)
    (`KismetArrayLibrary.Array_RemoveItem` (`/Game/ThirdPerson/Blueprints/BP_ThirdPersonCharacter.PlacedOrbs` (stale `Pickup` _asbp_third_person_character)) self)
    (`self.CalculateWalls`)
    (else
      (bind _asbp_third_person_character (cast `/Game/ThirdPerson/Blueprints/BP_ThirdPersonCharacter` (stale `self.PickupCollider.OnComponentBeginOverlap` OtherActor)))))
  (`self.K2_AttachToComponent` (`Character.Mesh` _asbp_third_person_character) "HandGrip_R" "SnapToTarget" "SnapToTarget" "KeepRelative" false)
  (set `self.CurrentPedestal` null))

(event `PlaceOnPedestal`
  (params (PedestalRef :type "/Game/MyBlueprints/BP_Pedestal Object Reference"))
  (if (`KismetSystemLibrary.IsValid` PedestalRef)
    (set `self.bIsHeld` false)
    (`self.K2_DetachFromActor` (stale `Pickup` _asbp_third_person_character) "KeepRelative" "KeepRelative" "KeepRelative")
    (`self.K2_AttachToComponent` (`self.GetComponentByClass` PedestalRef "/Script/Engine.SphereComponent") "None" "KeepRelative" "KeepRelative" "KeepRelative")
    (set `self.CurrentPedestal` PedestalRef)
    (`KismetArrayLibrary.Array_Add` (`/Game/ThirdPerson/Blueprints/BP_ThirdPersonCharacter.PlacedOrbs` (stale `Pickup` _asbp_third_person_character)) self)
    (`self.CalculateWalls`)))

(event `self.ReceiveBeginPlay`
  (bind _outactors (`GameplayStatics.GetAllActorsOfClass` "/Script/Engine.StaticMeshActor"))
  (for _array_element _outactors
    (if (`self.ActorHasTag` _array_element "PuzzleWall")
      (`KismetArrayLibrary.Array_Add` (`self.WallArray`) _array_element))))

(event `CalculateWalls`
  (`self.Color` (`/Game/ThirdPerson/Blueprints/BP_ThirdPersonCharacter.PlacedOrbs` (stale `Pickup` _asbp_third_person_character))))

(fn `Color`
  (params (placedOrbs :type "Array of /Game/MyBlueprints/BP_ObjectPickup Object Reference"))
  (returns (NewParam :type Boolean))
  (set `self.combined` 0)
  (for _array_element placedOrbs
    (if (`self.ActorHasTag` _array_element "Red")
      (set `self.combined` (+ (`self.combined`) 1)))
    (if (`self.ActorHasTag` _array_element "Green")
      (set `self.combined` (+ (`self.combined`) 2)))
    (if (`self.ActorHasTag` _array_element "Blue")
      (set `self.combined` (+ (`self.combined`) 4))))
  (`KismetSystemLibrary.PrintString` (`KismetStringLibrary.Conv_IntToString` (`self.combined`)))
  (switch `int` (`self.combined`)
    (:`0`
      (for _array_element_2 (`self.WallArray`)
        (`SceneComponent.SetVisibility` (`Actor.RootComponent` _array_element_2) true false)
        (`PrimitiveComponent.SetCollisionEnabled` (`StaticMeshActor.StaticMeshComponent` _array_element_2) "QueryAndPhysics"))
      (return false))
    (:`1`
      (for _array_element_3 (`self.WallArray`)
        (if (`self.ActorHasTag` _array_element_3 "Red")
          (bind _staticmeshcomponent (`StaticMeshActor.StaticMeshComponent` _array_element_3))
          (`SceneComponent.SetVisibility` _staticmeshcomponent false false)
          (`PrimitiveComponent.SetCollisionEnabled` _staticmeshcomponent "NoCollision")
          (else
            (`SceneComponent.SetVisibility` _staticmeshcomponent true false)
            (`PrimitiveComponent.SetCollisionEnabled` _staticmeshcomponent "QueryAndPhysics"))))
      (return false))
    (:`2`
      (for _array_element_4 (`self.WallArray`)
        (if (`self.ActorHasTag` _array_element_4 "Green")
          (bind _staticmeshcomponent_2 (`StaticMeshActor.StaticMeshComponent` _array_element_4))
          (`SceneComponent.SetVisibility` _staticmeshcomponent_2 false false)
          (`PrimitiveComponent.SetCollisionEnabled` _staticmeshcomponent_2 "NoCollision")
          (else
            (`SceneComponent.SetVisibility` _staticmeshcomponent_2 true false)
            (`PrimitiveComponent.SetCollisionEnabled` _staticmeshcomponent_2 "QueryAndPhysics"))))
      (return false))
    (:`3`
      (for _array_element_5 (`self.WallArray`)
        (if (`self.ActorHasTag` _array_element_5 "Yellow")
          (bind _staticmeshcomponent_3 (`StaticMeshActor.StaticMeshComponent` _array_element_5))
          (`SceneComponent.SetVisibility` _staticmeshcomponent_3 false false)
          (`PrimitiveComponent.SetCollisionEnabled` _staticmeshcomponent_3 "NoCollision")
          (else
            (`SceneComponent.SetVisibility` _staticmeshcomponent_3 true false)
            (`PrimitiveComponent.SetCollisionEnabled` _staticmeshcomponent_3 "QueryAndPhysics"))))
      (return false))
    (:`4`
      (for _array_element_6 (`self.WallArray`)
        (if (`self.ActorHasTag` _array_element_6 "Blue")
          (bind _staticmeshcomponent_4 (`StaticMeshActor.StaticMeshComponent` _array_element_6))
          (`SceneComponent.SetVisibility` _staticmeshcomponent_4 false false)
          (`PrimitiveComponent.SetCollisionEnabled` _staticmeshcomponent_4 "NoCollision")
          (else
            (`SceneComponent.SetVisibility` _staticmeshcomponent_4 true false)
            (`PrimitiveComponent.SetCollisionEnabled` _staticmeshcomponent_4 "QueryAndPhysics"))))
      (return false))
    (:`5`
      (for _array_element_7 (`self.WallArray`)
        (if (`self.ActorHasTag` _array_element_7 "Pink")
          (bind _staticmeshcomponent_5 (`StaticMeshActor.StaticMeshComponent` _array_element_7))
          (`SceneComponent.SetVisibility` _staticmeshcomponent_5 false false)
          (`PrimitiveComponent.SetCollisionEnabled` _staticmeshcomponent_5 "NoCollision")
          (else
            (`SceneComponent.SetVisibility` _staticmeshcomponent_5 true false)
            (`PrimitiveComponent.SetCollisionEnabled` _staticmeshcomponent_5 "QueryAndPhysics"))))
      (return false))
    (:`6`
      (for _array_element_8 (`self.WallArray`)
        (if (`self.ActorHasTag` _array_element_8 "Cyan")
          (bind _staticmeshcomponent_6 (`StaticMeshActor.StaticMeshComponent` _array_element_8))
          (`SceneComponent.SetVisibility` _staticmeshcomponent_6 false false)
          (`PrimitiveComponent.SetCollisionEnabled` _staticmeshcomponent_6 "NoCollision")
          (else
            (`SceneComponent.SetVisibility` _staticmeshcomponent_6 true false)
            (`PrimitiveComponent.SetCollisionEnabled` _staticmeshcomponent_6 "QueryAndPhysics"))))
      (return false))
    (:`7`
      (for _array_element_9 (`self.WallArray`)
        (if (`self.ActorHasTag` _array_element_9 "White")
          (bind _staticmeshcomponent_7 (`StaticMeshActor.StaticMeshComponent` _array_element_9))
          (`SceneComponent.SetVisibility` _staticmeshcomponent_7 false false)
          (`PrimitiveComponent.SetCollisionEnabled` _staticmeshcomponent_7 "NoCollision")
          (else
            (`SceneComponent.SetVisibility` _staticmeshcomponent_7 true false)
            (`PrimitiveComponent.SetCollisionEnabled` _staticmeshcomponent_7 "QueryAndPhysics"))))
      (return false))
    (:`8`
      (return false))))

(fn `UserConstructionScript`)